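; First-person player character that recreates the SUPERHOT mechanic where time moves only when the player moves.
; Each tick, global time dilation is full speed when the sum of the stored movement axes is nonzero and near-frozen otherwise, so opposite-signed axes can cancel.
; Inputs drive yaw-relative movement, look and jump.
; Shooting spawns a SuperHotBullet at the gun and applies an impulse along the camera's forward vector.
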(event EventBeginPlay)

(event Collision|EventActorBeginOverlap
  (params (OtherActor :type Actor%20Object%20Reference)))

(event EventTick
  (params (DeltaSeconds :type Float%20%28single-precision%29))
  ;[1 1 1] Bullet Time
  (if (!= (+ (Variables|Default|GetHAxis) (Variables|Default|GetVAxis)) 0.0)
    (Utilities|Time|SetGlobalTimeDilation 1.0)
    (else
      (Utilities|Time|SetGlobalTimeDilation 0.05))))

(event Input|ActionEvents|InputActionJump
  (params (Key :type Key%20Structure))
  (:Pressed
    (Character|Jump)))

(event Input|ActionEvents|InputActionShoot
  (params (Key :type Key%20Structure))
  ;[1 1 1] Shoot Bullet
  (:Pressed
    (bind _returnvalue (Game|SpawnActorfromClass "/Game/Blueprints/SuperHot/SuperHotBullet.SuperHotBullet_C" (Transformation|GetWorldTransform (Variables|Default|GetGun)) "Undefined" 0 0))
    (Physics|AddImpulse (Variables|/Game/Blueprints/SuperHot/SuperHotBullet.SuperHotBullet_C|GetCube _returnvalue) (* (Math|Vector|GetForwardVector (Transformation|GetWorldRotation (Variables|Default|GetCamera))) (Variables|Default|GetBullet%20Speed)) "None" false)))

(event Input|AxisEvents|InputAxisMouseLookHorizontal
  (params (AxisValue :type Float%20%28single-precision%29))
  (Pawn|Input|AddControllerYawInput AxisValue))

(event Input|AxisEvents|InputAxisHorizontal
  (params (AxisValue :type Float%20%28single-precision%29))
  (Pawn|Input|AddMovementInput (Math|Vector|GetRightVector (Math|Rotator|MakeRotator 0.0 0.0 (.yaw (Pawn|GetControlRotation :!class /Script/Engine.Pawn)))) AxisValue false)
  (Variables|Default|SetHAxis AxisValue))

(event Input|AxisEvents|InputAxisVertical
  (params (AxisValue :type Float%20%28single-precision%29))
  (Pawn|Input|AddMovementInput (Math|Vector|GetForwardVector (Math|Rotator|MakeRotator 0.0 0.0 (.yaw (Pawn|GetControlRotation :!class /Script/Engine.Pawn)))) AxisValue false)
  (Variables|Default|SetVAxis AxisValue))

(event Input|AxisEvents|InputAxisMouseLookVertical
  (params (AxisValue :type Float%20%28single-precision%29))
  (Pawn|Input|AddControllerPitchInput AxisValue))

(fn ConstructionScript)