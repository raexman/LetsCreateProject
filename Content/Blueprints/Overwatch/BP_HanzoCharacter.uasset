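; Player character modeled on Overwatch's Hanzo, with mouse look, camera-yaw-relative movement, double jump, directional dash and wall climbing.
; A DoN counter, reset on landing, selects jump or upward launch, while the dash launches along the camera with zero ground friction, then stops and recovers.
; Each Tick, a line trace finds tagged walls and launches upward while Space is held, up to a time limit, locking mouse look.
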(event EventBeginPlay)

(event Collision|EventActorBeginOverlap
  (params (OtherActor :type Actor%20Object%20Reference)))

(event EventOnLanded
  (params (Hit :type Hit%20Result%20Structure%20%28by%20ref%29))
  ;[1 1 1] Double Jump
  (Variables|Flags|SetCan%20Wall%20Climb true)
  (Utilities|FlowControl|DoN 2) ; enters at Reset
)

(event EventTick
  (params (DeltaSeconds :type Float%20%28single-precision%29))
  (CallFunction|AttemptWallClimb))

(event Input|ActionEvents|InputActionJump
  (params (Key :type Key%20Structure))
  ;[1 1 1] Double Jump
  (:Pressed
    (bind _counter (Utilities|FlowControl|DoN 2)
      (:Exit
        (switch int _counter
          (:1
            (Character|Jump))
          (:2
            (Character|LaunchCharacter (Math|Vector|MakeVector 0.0 0.0 (Variables|Default|GetDouble%20Jump%20Distance)) false true)))))))

(event Input|ActionEvents|InputActionDash
  (params (Key :type Key%20Structure))
  ;[1 1 1] Dash
  (:Pressed
    (if (Variables|Flags|GetCan%20Dash)
      (Variables|/Script/Engine.CharacterMovementComponent|SetGroundFriction (Variables|Character|GetCharacterMovement) 0.0)
      (Character|LaunchCharacter (* (Math|Vector|GetForwardVector (Variables|Default|GetCamera)) (Variables|Dash|GetDash%20Velocity)) false false)
      (Utilities|FlowControl|Delay (Variables|Dash|GetDash%20Duration))
      (Variables|Flags|SetCan%20Dash false)
      (Components|Movement|StopMovementImmediately (Variables|Character|GetCharacterMovement))
      (Variables|/Script/Engine.CharacterMovementComponent|SetGroundFriction (Variables|Character|GetCharacterMovement) 8.0)
      (Utilities|FlowControl|Delay (Variables|Dash|GetDash%20Recovery))
      (Variables|Flags|SetCan%20Dash true))))

(event Input|AxisEvents|InputAxisMouseLookHorizontal
  (params (AxisValue :type Float%20%28single-precision%29))
  (if (== (Variables|WallClimb|GetClimb%20Time) 0.0)
    (Pawn|Input|AddControllerYawInput AxisValue)))

(event Input|AxisEvents|InputAxisHorizontal
  (params (AxisValue :type Float%20%28single-precision%29))
  (Pawn|Input|AddMovementInput (Math|Vector|GetRightVector (Math|Rotator|MakeRotator 0.0 0.0 (.yaw (Pawn|GetControlRotation :!class /Script/Engine.Pawn)))) AxisValue false))

(event Input|AxisEvents|InputAxisVertical
  (params (AxisValue :type Float%20%28single-precision%29))
  (Pawn|Input|AddMovementInput (Math|Vector|GetForwardVector (Math|Rotator|MakeRotator 0.0 0.0 (.yaw (Pawn|GetControlRotation :!class /Script/Engine.Pawn)))) AxisValue false))

(event Input|AxisEvents|InputAxisMouseLookVertical
  (params (AxisValue :type Float%20%28single-precision%29))
  (if (== (Variables|WallClimb|GetClimb%20Time) 0.0)
    (Pawn|Input|AddControllerPitchInput AxisValue)))

(fn ConstructionScript)

(fn AttemptWallClimb
  (bind _outhit (Collision|LineTraceByChannel (Transformation|GetActorLocation) (Transformation|GetWorldLocation (Variables|Default|GetLineEndLocation)) "TraceTypeQuery1" false 0 "ForDuration"))
  (if (Utilities|IsValid (.hitactor _outhit))
    (if (and (Actor|ActorHasTag (.hitactor _outhit) (Variables|Tags|GetClimbable%20Tag)) (Variables|Flags|GetCan%20Wall%20Climb))
      (bind _output_get (Variables|WallClimb|SetClimb%20Time (Class|PlayerController|GetInputKeyTimeDown (Game|GetPlayerController 0) "SpaceBar")))
      (if (!= _output_get 0.0)
        (if (<= _output_get (Variables|WallClimb|GetClimb%20Duration))
          (Character|LaunchCharacter (Math|Vector|MakeVector 0.0 0.0 (Variables|WallClimb|GetClimb%20Speed)) true true)
          (return true)
          (else
            (Variables|Flags|SetCan%20Wall%20Climb false) ; If we reached Climb Duration, stop climbing and reset the can climb flag
          )))
      (else
        (Variables|WallClimb|SetClimb%20Time 0.0 :!label _label) ; Reset Climb Time
      ))
    (else
      (goto _label)))
  (return false))