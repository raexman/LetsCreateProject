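; Player character modelled on Overwatch's Widowmaker, with basic move and look input and a grappling hook ability.
; The ability line-traces from the actor along the camera's forward vector, rejecting misses and physics-simulating targets.
; A valid hit animates the rope by timeline interpolation and launches the character upward, then toward the hook point, before a recovery delay.
; While grappling, jumping damps velocity and hitting physics-simulating components pops the character upward.
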(event OnComponentHit(CapsuleComponent)
  (params (HitComponent :type Primitive%20Component%20Object%20Reference) (OtherActor :type Actor%20Object%20Reference) (OtherComp :type Primitive%20Component%20Object%20Reference) (NormalImpulse :type Vector :default "0, 0, 0") (Hit :type Hit%20Result%20Structure%20%28by%20ref%29))
  (if (Physics|IsSimulatingPhysics OtherComp "None")
    (if (Variables|Default|GetGrapple%20Hook%20Enabled)
      (Character|LaunchCharacter "0, 0,400.000000" true true))))

(event Custom|Shoot%20Grapple%20Hook
  (bind _grapple_rope (Variables|Default|GetGrapple%20Rope))
  (Rendering|SetVisibility _grapple_rope true false)
  (bind _interpspeed (Timeline|Grapple%20Hook%20Shooting%20Timeline PlayFromStart)
    (:Update
      (Transformation|SetWorldLocation (Variables|Default|GetGrapple%20Rope) (Math|Interpolation|VInterpTo (Transformation|GetWorldLocation _grapple_rope) (Variables|Default|GetHook%20Location) (Variables|Default|GetDelta%20Time) _interpspeed) false false))))

(event Custom|Reset%20Grapple%20Hook
  (Rendering|SetVisibility (Variables|Default|GetGrapple%20Rope) false false)
  (Variables|Default|SetGrapple%20Hook%20Enabled false)
  (Utilities|FlowControl|Delay (Variables|Default|GetGrapple%20Hook%20Recovery))
  (Variables|Default|SetCan%20Grapple%20Hook true))

(event EventBeginPlay)

(event Collision|EventActorBeginOverlap
  (params (OtherActor :type Actor%20Object%20Reference)))

(event EventTick
  (params (DeltaSeconds :type Float%20%28single-precision%29))
  ;[1 1 1] Set Delta Time
  (Variables|Default|SetDelta%20Time DeltaSeconds))

(event Input|ActionEvents|InputActionJump
  (params (Key :type Key%20Structure))
  (bind _charactermovement (Variables|Character|GetCharacterMovement))
  (:Pressed
    (if (Variables|Default|GetGrapple%20Hook%20Enabled)
      (Variables|/Script/Engine.MovementComponent|SetVelocity _charactermovement (* (Variables|/Script/Engine.MovementComponent|GetVelocity _charactermovement) 0.66)))
    (Character|Jump)))

(event Input|ActionEvents|InputActionAbility
  (params (Key :type Key%20Structure))
  (bind _returnvalue (Transformation|GetActorLocation))
  (:Pressed
    (if (Variables|Default|GetCan%20Grapple%20Hook)
      (Variables|Default|SetCan%20Grapple%20Hook false)
      (Variables|Default|SetGrapple%20Hook%20Enabled true)
      (bind (_outhit _returnvalue_2) (Collision|LineTraceByChannel _returnvalue (+ _returnvalue (* (Math|Vector|GetForwardVector (Variables|Default|GetCamera)) (Variables|Default|GetGrapple%20Hook%20Distance))) "TraceTypeQuery1" false 0 "ForDuration"))
      (if _returnvalue_2
        (if (Physics|IsSimulatingPhysics (.HitComponent (Collision|BreakHitResult _outhit)) "None")
          (CallFunction|ResetGrappleHook :!label _label)
          (else
            (Variables|Default|SetHook%20Location (.Location (Collision|BreakHitResult _outhit)))
            (CallFunction|ShootGrappleHook)
            (Character|LaunchCharacter "0, 0,500.000000" true true)
            (Utilities|FlowControl|Delay 0.2)
            (Character|LaunchCharacter (* (Math|Vector|Normalize (- (Variables|Default|GetHook%20Location) (Transformation|GetActorLocation))) (Variables|Default|GetGrapple%20Hook%20Velocity)) false false)
            (Utilities|FlowControl|Delay 0.4)
            (CallFunction|ResetGrappleHook)))
        (else
          (goto _label))))))

(event Input|AxisEvents|InputAxisMouseLookHorizontal
  (params (AxisValue :type Float%20%28single-precision%29))
  (Pawn|Input|AddControllerYawInput AxisValue))

(event Input|AxisEvents|InputAxisHorizontal
  (params (AxisValue :type Float%20%28single-precision%29))
  (Pawn|Input|AddMovementInput (Math|Vector|GetRightVector (Math|Rotator|MakeRotator 0.0 0.0 (.yaw (Pawn|GetControlRotation :!class /Script/Engine.Pawn)))) AxisValue false))

(event Input|AxisEvents|InputAxisVertical
  (params (AxisValue :type Float%20%28single-precision%29))
  (Pawn|Input|AddMovementInput (Math|Vector|GetForwardVector (Math|Rotator|MakeRotator 0.0 0.0 (.yaw (Pawn|GetControlRotation :!class /Script/Engine.Pawn)))) AxisValue false))

(event Input|AxisEvents|InputAxisMouseLookVertical
  (params (AxisValue :type Float%20%28single-precision%29))
  (Pawn|Input|AddControllerPitchInput AxisValue))

(fn ConstructionScript)