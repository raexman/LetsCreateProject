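; Player character Blueprint for an Overwatch-style Pharah, with mouse look, yaw-relative movement, a jetpack hover and a vertical boost.
; Jump starts a timeline that applies upward impulses while polled Space Bar is held and HoverTime is within its limit.
; Each update raises HoverTime while held or lowers it when released, and the timeline replays until it drains.
; Dash launches the character upward, then a delay gates the next boost.
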(event EventBeginPlay)

(event Collision|EventActorBeginOverlap
  (params (OtherActor :type Actor%20Object%20Reference)))

(event Input|ActionEvents|InputActionJump
  (params (Key :type Key%20Structure))
  (bind _returnvalue (Game|GetPlayerController 0))
  (:Pressed
    (Timeline|Hover%20Timeline Play
      (:Update
        (Utilities|FlowControl|Sequence
          (:then_0
            (if (> (Class|PlayerController|GetInputKeyTimeDown _returnvalue "SpaceBar") 0.0)
              (if (<= (Variables|Default|GetHover%20Time) (Variables|Default|GetMax%20Hover%20Time))
                (Physics|AddImpulse (Variables|Character|GetCharacterMovement) (Math|Vector|MakeVector 0.0 0.0 (Variables|Default|GetHover%20Velocity)) false))))
          (:then_1
            (if (Math|Float|NearlyEqual(Float) (Class|PlayerController|GetInputAnalogKeyState _returnvalue "SpaceBar") 0.0 1e-06)
              (if (> (Variables|Default|GetHover%20Time) 0.0)
                (Math|Float|DecrementFloat (Variables|Default|GetHover%20Time)))
              (elif (<= (Variables|Default|GetHover%20Time) (Variables|Default|GetMax%20Hover%20Time))
                (Math|Float|IncrementFloat (Variables|Default|GetHover%20Time)))))))
      (:Finished
        (if (> (Variables|Default|GetHover%20Time) 0.0)
          (Timeline|Hover%20Timeline Play))))))

(event Input|ActionEvents|InputActionDash
  (params (Key :type Key%20Structure))
  ;[1 1 1] Boost
  (:Pressed
    (if (Variables|Default|GetCan%20Boost)
      (Variables|Default|SetCan%20Boost false)
      (Character|LaunchCharacter (Math|Vector|MakeVector 0.0 0.0 (Variables|Default|GetBoost%20Velocity)) false true)
      (Utilities|FlowControl|Delay (Variables|Default|GetBoost%20Recovery))
      (Variables|Default|SetCan%20Boost true))))

(event Input|AxisEvents|InputAxisMouseLookHorizontal
  (params (AxisValue :type Float%20%28single-precision%29))
  (Pawn|Input|AddControllerYawInput AxisValue))

(event Input|AxisEvents|InputAxisHorizontal
  (params (AxisValue :type Float%20%28single-precision%29))
  (Pawn|Input|AddMovementInput (Math|Vector|GetRightVector (Math|Rotator|MakeRotator 0.0 0.0 (.yaw (Pawn|GetControlRotation :!class /Script/Engine.Pawn)))) AxisValue false))

(event Input|AxisEvents|InputAxisVertical
  (params (AxisValue :type Float%20%28single-precision%29))
  (Pawn|Input|AddMovementInput (Math|Vector|GetForwardVector (Math|Rotator|MakeRotator 0.0 0.0 (.yaw (Pawn|GetControlRotation :!class /Script/Engine.Pawn)))) AxisValue false))

(event Input|AxisEvents|InputAxisMouseLookVertical
  (params (AxisValue :type Float%20%28single-precision%29))
  (Pawn|Input|AddControllerPitchInput AxisValue))

(fn ConstructionScript)