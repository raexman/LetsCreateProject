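; Player character modeled on Overwatch's Tracer, with first-person movement inputs, a charge-based Blink and a Recall rewind.
; Tick records transforms at intervals with debug frustums, dropping the newest entry when full, and recharges Blink charges.
; Recall disables collision and gravity, then lerps location and control rotation backward through the recorded transforms.
; Blink launches horizontally along camera forward without gravity, then stops after a short duration.
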(event EventBeginPlay)

(event Collision|EventActorBeginOverlap
  (params (OtherActor :type Actor%20Object%20Reference)))

(event EventTick
  (params (DeltaSeconds :type Float%20%28single-precision%29))
  (bind _returnvalue (Game|GetPlayerController 0))
  (bind _recall_positions (Variables|Default|GetRecall%20Positions))
  (bind _recall_positions_2 (Variables|Default|GetRecall%20Positions))
  (Variables|Default|SetDelta%20Time DeltaSeconds)
  (Utilities|FlowControl|Sequence
    (:then_0
      ;[1 1 1] Register Positions
      (if (Variables|Default|GetCan%20Set%20Position)
        (Utilities|FlowControl|Delay (Variables|Default|GetPosition%20Register%20Rate))
        (if (>= (Utilities|Array|Length _recall_positions_2) (Variables|Default|GetRecall%20Positions%20Size))
          (Utilities|Array|RemoveIndex _recall_positions_2 (Utilities|Array|LastIndex _recall_positions_2))
          (else
            (bind _returnvalue_2 (Utilities|Array|Add _recall_positions (Transformation|GetActorTransform)))
            (Class|KismetSystemLibrary|DrawDebugFrustum (Utilities|Array|Get(acopy) _recall_positions _returnvalue_2) "(R=1.000000,G=0.292484,B=0.000000,A=1.000000)" 6.0 15.0)))
        (else
          ;[1 1 1] Recall
          (if (Variables|Default|GetRecall%20Pressed)
            (Transformation|SetActorLocation (.location (Math|Transform|Lerp(Transform) (Transformation|GetActorTransform) (Utilities|Array|Get(acopy) (Variables|Default|GetRecall%20Positions) (Variables|Default|GetCounter)) (* (Variables|Default|GetDelta%20Time) (Variables|Default|GetTravel%20Speed)))) false false)
            (Pawn|SetControlRotation _returnvalue (Math|Rotator|Lerp(Rotator) (Transformation|GetActorRotation _returnvalue) (.rotation (Math|Transform|Lerp(Transform) (Transformation|GetActorTransform) (Utilities|Array|Get(acopy) (Variables|Default|GetRecall%20Positions) (Variables|Default|GetCounter)) (* (Variables|Default|GetDelta%20Time) (Variables|Default|GetTravel%20Speed)))) (* (Variables|Default|GetDelta%20Time) (Variables|Default|GetRotation%20Speed))))
            (if (Class|KismetMathLibrary|NearlyEqualTransformTransform (Transformation|GetActorTransform) (Utilities|Array|Get(acopy) (Variables|Default|GetRecall%20Positions) (Variables|Default|GetCounter)) 1.2e+02 1.2e+02 1.2e+02)
              (if (== (Variables|Default|GetCounter) 0)
                (Variables|Default|SetCan%20Set%20Position true)
                (Variables|Default|SetRecall%20Pressed false)
                (Utilities|Array|Clear (Variables|Default|GetRecall%20Positions))
                (Collision|SetActorEnableCollision true)
                (Variables|/Script/Engine.CharacterMovementComponent|SetGravityScale (Variables|Character|GetCharacterMovement) 1.0)
                (Utilities|FlowControl|Delay (Variables|Default|GetRecall%20Recovery))
                (Variables|Default|SetCan%20Recall true)
                (else
                  (Math|Integer|DecrementInt (Variables|Default|GetCounter)))))))))
    (:then_1
      ;[1 1 1] Blink Charges
      (if (< (Variables|Default|GetBlink%20Charges) (Variables|Default|GetMax%20Blink%20Charges))
        (bind _output_get (Variables|Default|SetBlink%20Recharge%20Timer (+ (Variables|Default|GetDelta%20Time) (Variables|Default|GetBlink%20Recharge%20Timer))))
        (if (>= _output_get (Variables|Default|GetBlink%20Recharge%20Rate))
          (Math|Integer|IncrementInt (Variables|Default|GetBlink%20Charges)
            (:%20%20
              (Variables|Default|SetBlink%20Recharge%20Timer 0.0))))))))

(event Input|ActionEvents|InputActionJump
  (params (Key :type Key%20Structure))
  (:Pressed
    (Character|Jump)))

(event Input|ActionEvents|InputActionAbility
  (params (Key :type Key%20Structure))
  ;[1 1 1] Recall
  (:Pressed
    (if (Variables|Default|GetCan%20Recall)
      (Collision|SetActorEnableCollision false)
      (Variables|/Script/Engine.CharacterMovementComponent|SetGravityScale (Variables|Character|GetCharacterMovement) 0.0)
      (Variables|Default|SetRecall%20Pressed true)
      (Variables|Default|SetCan%20Recall false)
      (Variables|Default|SetCan%20Set%20Position false)
      (Variables|Default|SetCounter (Utilities|Array|LastIndex (Variables|Default|GetRecall%20Positions))))))

(event Input|ActionEvents|InputActionDash
  (params (Key :type Key%20Structure))
  (bind _camera (Variables|Default|GetCamera))
  (bind _returnvalue (Math|Vector|GetForwardVector _camera))
  ;[1 1 1] Blink
  (:Pressed
    (if (> (Variables|Default|GetBlink%20Charges) 0)
      (if (Variables|Default|GetCan%20Blink)
        (Variables|/Script/Engine.CharacterMovementComponent|SetGravityScale (Variables|Character|GetCharacterMovement) 0.0)
        (Character|LaunchCharacter (* (Math|Vector|MakeVector (.x _returnvalue) (.y _returnvalue) 0.0) (Variables|Default|GetBlink%20Velocity)) false false)
        (Utilities|FlowControl|Delay (Variables|Default|GetBlink%20Duration))
        (Variables|Default|SetCan%20Blink false)
        (Components|Movement|StopMovementImmediately (Variables|Character|GetCharacterMovement))
        (Variables|/Script/Engine.CharacterMovementComponent|SetGravityScale (Variables|Character|GetCharacterMovement) 1.0)
        (Utilities|FlowControl|Delay (Variables|Default|GetBlink%20Recovery))
        (Variables|Default|SetCan%20Blink true)
        (Math|Integer|DecrementInt (Variables|Default|GetBlink%20Charges))))))

(event Input|AxisEvents|InputAxisMouseLookHorizontal
  (params (AxisValue :type Float%20%28single-precision%29))
  (Pawn|Input|AddControllerYawInput AxisValue))

(event Input|AxisEvents|InputAxisHorizontal
  (params (AxisValue :type Float%20%28single-precision%29))
  (Pawn|Input|AddMovementInput (Math|Vector|GetRightVector (Math|Rotator|MakeRotator 0.0 0.0 (.yaw (Pawn|GetControlRotation :!class /Script/Engine.Pawn)))) AxisValue false))

(event Input|AxisEvents|InputAxisVertical
  (params (AxisValue :type Float%20%28single-precision%29))
  (Pawn|Input|AddMovementInput (Math|Vector|GetForwardVector (Math|Rotator|MakeRotator 0.0 0.0 (.yaw (Pawn|GetControlRotation :!class /Script/Engine.Pawn)))) AxisValue false))

(event Input|AxisEvents|InputAxisMouseLookVertical
  (params (AxisValue :type Float%20%28single-precision%29))
  (Pawn|Input|AddControllerPitchInput AxisValue))

(fn ConstructionScript)